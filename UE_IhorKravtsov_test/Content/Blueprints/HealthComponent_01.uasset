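; Health component that tracks its owning actor's health as it takes damage.
; On BeginPlay it binds to the owner's OnTakeAnyDamage and sets health to the maximum.
; Each hit subtracts damage without clamping and broadcasts current and max health through the OnHealthChanges dispatcher.
; Damage and death only print debug strings, with no further death handling.
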(event Custom|onAnyDamage
  (params (DamagedActor :type Actor%20Object%20Reference) (Damage :type Float%20%28single-precision%29) (DamageType :type Damage%20Type%20Object%20Reference) (InstigatedBy :type Controller%20Object%20Reference) (DamageCauser :type Actor%20Object%20Reference))
  (Development|PrintString "DAMAGE" true true "(R=1.000000,G=0.029155,B=0.017787,A=1.000000)")
  (bind _output_get (Variables|Default|SetHealth_01 (- (Variables|Default|GetHealth_01) Damage)))
  (Default|CallOnHealthChanges _output_get (Variables|Default|GetMaxHealth_01))
  (if (<= _output_get 0.0)
    (Development|PrintString "DEAD")))

(event EventBeginPlay
  (EventDispatchers|BindEventtoOnTakeAnyDamage (Components|GetOwner) (delegate Custom|onAnyDamage))
  (Variables|Default|SetHealth_01 (Variables|Default|GetMaxHealth_01)))