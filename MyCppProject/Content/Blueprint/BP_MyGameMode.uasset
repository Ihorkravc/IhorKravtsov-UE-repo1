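; Game mode that sets the player character's starting health from a GameHealthSettings object.
; On BeginPlay, after a short delay, it passes the settings' StartHealth to the first player's BP_PlayerCharacter and prints the value.
; ApplyHealthSettings stores new settings and immediately reapplies their starting health, casting to GAPlayerCharacter instead of the Blueprint class.
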(event EventBeginPlay
  (bind _gamehealthsettings (Variables|Default|GetGameHealthSettings))
  (bind _starthealth (Variables|/Game/Blueprint/DA_GameModeSettings.DA_GameModeSettings_C|GetStartHealth _gamehealthsettings))
  (Utilities|IsValid (Variables|Default|GetGameHealthSettings)
    (:Is%20Valid
      (if true
        (Utilities|FlowControl|Delay 0.1)
        (bind _asbp_player_character (Utilities|Casting|CastToBP_PlayerCharacter (Game|GetPlayerCharacter 0)))
        (Class|GABaseCharacter|SetInitialHealth _asbp_player_character _starthealth)
        (Development|PrintString (Utilities|String|ToString(Text) (Utilities|Text|FormatText "{A}" (Utilities|Text|ToText(Float) _starthealth "HalfToEven"))))))))

(event EventTick
  (params (DeltaSeconds :type Float%20%28single-precision%29)))

(fn ConstructionScript)

(fn ApplyHealthSettings
  (params (NewSettings :type DA%20Game%20Mode%20Settings%20Object%20Reference))
  (Utilities|IsValid NewSettings
    (:Is%20Valid
      (if true
        (bind _asgaplayer_character (Utilities|Casting|CastToGAPlayerCharacter (Game|GetPlayerCharacter 0)))
        (Variables|Default|SetGameHealthSettings NewSettings)
        (Class|GABaseCharacter|SetInitialHealth _asgaplayer_character (Variables|/Game/Blueprint/DA_GameModeSettings.DA_GameModeSettings_C|GetStartHealth NewSettings))))))